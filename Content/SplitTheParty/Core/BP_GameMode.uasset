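; BP_GameMode runs the turn-based hero game on a hex map, spawning Knight, Bard and Sage heroes and showing the game-over screen.
; Each turn start refreshes every tile's available actions from the current hero.
; Selected actions move, quest or rest, with click events disabled during movement.
; Turns finish after movement, rest or dismissal of a quest dialog, which commits effects when a peril was found.
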(event Custom|OnActionSelected
  (params (HexTile :type BP%20Hex%20Tile%20Object%20Reference) (Action :type EHexAction%20Enum :default "Move"))
  (bind _returnvalue (Game|GetPlayerController 0))
  (bind _currenthero (Variables|Default|GetCurrentHero))
  (bind _asbp_hero (Utilities|Casting|CastToBP_Hero _currenthero))
  (bind _asbp_player_controller (Utilities|Casting|CastToBP_PlayerController _returnvalue))
  ;[1 1 1] Respond to hex selection. If it's a neighbor, move. If it's the hero's tile, quest or rest.
  (switch Utilities|FlowControl|Switch|SwitchonEHexAction Action
    (:Move
      (Variables|/Script/Engine.PlayerController|SetbEnableClickEvents (Game|GetPlayerController 0) false)
      (Class|Hero|Moveto _asbp_hero HexTile))
    (:Quest
      (bind _returnvalue_2 (Class|Hero|Quest _asbp_hero))
      (if (Utilities|IsValid (Variables|/Script/SplitTheParty.QuestResult|GetPeril _returnvalue_2))
        (bind _returnvalue_3 (UserInterface|CreateWidget "/Game/SplitTheParty/UI/WBP_Questing.WBP_Questing_C" _returnvalue _returnvalue_2))
        (EventDispatchers|BindEventtoOnDialogDismissed _returnvalue_3 (delegate Custom|OnDialogDismissed))
        (Default|ShowDialogBox _asbp_player_controller _returnvalue_3)
        (else
          (bind _returnvalue_4 (UserInterface|CreateWidget "/Game/SplitTheParty/UI/WBP_NoQuestHere.WBP_NoQuestHere_C" _returnvalue))
          (EventDispatchers|BindEventtoOnDialogDismissed _returnvalue_4 (delegate Custom|OnDialogDismised))
          (Default|ShowDialogBox _asbp_player_controller _returnvalue_4))))
    (:Rest
      (Class|Hero|Rest _asbp_hero)
      (Class|SplitthePartyGameMode|FinishHeroTurn))))

(event Custom|OnDialogDismissed
  (params (Dialog :type WBP%20Dismissable%20Dialog%20Object%20Reference))
  (Class|QuestResult|CommitEffects (stale Custom|OnActionSelected _returnvalue_2))
  (Class|SplitthePartyGameMode|FinishHeroTurn))

(event Custom|OnDialogDismised
  (params (Dialog :type WBP%20Dismissable%20Dialog%20Object%20Reference))
  (Class|SplitthePartyGameMode|FinishHeroTurn))

(event EventEndGame
  (bind _returnvalue (Game|GetPlayerController 0))
  ;[1 1 1] End Game: Show the end game stats.
  (bind _returnvalue_2 (UserInterface|CreateWidget "/Game/SplitTheParty/UI/WBP_GameOver.WBP_GameOver_C" _returnvalue))
  (Default|ShowDialogBox (.AsBP%20Player%20Controller (Utilities|Casting|CastToBP_PlayerController _returnvalue)) _returnvalue_2))

(event EventStartTurn
  ;[1 1 1] Start Turn: Update all the actions on the tiles
  (bind _outactors (Actor|GetAllActorsOfClass "/Game/SplitTheParty/Board/BP_HexTile.BP_HexTile_C"))
  (for _array_element _outactors
    (Class|HexTile|SetTileActions _array_element (Class|Hero|DeterminePossibleActions (Variables|Default|GetCurrentHero) _array_element))))

(event EventOnHeroMovementComplete
  ;[1 1 1] OnHeroMovementComplete: Check for agents and finish turn
  (|CallParentFunction)
  (Variables|/Script/Engine.PlayerController|SetbEnableClickEvents (Game|GetPlayerController 0) true)
  (Class|SplitthePartyGameMode|FinishHeroTurn))

(event EventSpawnHeroonTile
  (params (index :type Integer) (Tile :type Hex%20Tile%20Object%20Reference))
  (bind _asbp_hex_tile (Utilities|Casting|CastToBP_HexTile Tile))
  ;[1 1 1] Spawn a hero
  (Game|SpawnActorfromClass "/Game/SplitTheParty/Board/BP_Hero.BP_Hero_C" (Math|Transform|MakeTransform (Transformation|GetSocketLocation (Variables|/Game/SplitTheParty/Board/BP_HexTile.BP_HexTile_C|GetHexMesh _asbp_hex_tile) (Utilities|String|StringToName (Utilities|String|Append "Hero" (Utilities|String|ToString(Integer) index)))) "0, 0, 0" "1,1,1") "Undefined" 0 index _asbp_hex_tile (Utilities|Select :Index index :Option%200 "(R=1.000000,G=0.000000,B=0.000000,A=1.000000)" :Option%201 "(R=0.000000,G=0.000000,B=1.000000,A=1.000000)" :Option%202 "(R=0.000000,G=1.000000,B=0.000000,A=1.000000)") (Utilities|Select :Index index :Option%200 "Knight" :Option%201 "Bard" :Option%202 "Sage") 0))

(fn ConstructionScript)

(fn GetPerilatHeroLocation
  (params (Hero :type Hero%20Object%20Reference))
  (return (Variables|/Script/SplitTheParty.HexTile|GetPeril (Class|WorldMap|GetTile (Variables|Default|GetWorldMap) (Variables|/Script/SplitTheParty.HexTile|GetCoordinates (Variables|/Script/SplitTheParty.Hero|GetTile Hero))))))