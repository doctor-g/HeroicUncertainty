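; Player controller for Split The Party that creates the HUD and manages modal dialog boxes, including rumor reports and a quit confirmation.
; ShowDialogBox adds a dialog, switches input to UI-only and binds its dismissal event.
; Timelines scale dialogs on show and dismissal, after which the dialog is removed and game-and-UI input restored.
; Rumor reports show overrides if any hero on the agent's tile reveals them, queried through BP_GameMode.
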(event Custom|ZoomDialog
  (params (Dialog :type WBP%20Dismissable%20Dialog%20Object%20Reference))
  (bind _percent (Timeline|DialogZoom PlayFromStart)
    (:Update
      (Widget|Transform|SetRenderScale Dialog (Math|Vector2D|MakeVector2D _percent _percent)))))

(event Custom|OnDialogDismissed
  (params (Dialog :type WBP%20Dismissable%20Dialog%20Object%20Reference))
  (EventDispatchers|UnbindEventfromOnDialogDismissed Dialog (delegate Custom|OnDialogDismissed))
  (bind _percent (Timeline|DialogZoomOut PlayFromStart)
    (:Update
      (Widget|Transform|SetRenderScale Dialog (Math|Vector2D|MakeVector2D _percent _percent)))
    (:Finished
      (Widget|RemovefromParent Dialog)
      (Input|SetInputModeGameandUI self 0 "DoNotLock" true))))

(event EventBeginPlay
  ;[1 1 1] BeginPlay: Construct the HUD
  (bind _returnvalue (UserInterface|CreateWidget "/Game/SplitTheParty/UI/WBP_HUD.WBP_HUD_C" self))
  (UserInterface|Viewport|AddtoViewport _returnvalue 0))

(event EventShowRumorReport
  (params (Agent :type Agent%20Object%20Reference))
  ;[1 1 1] Show rumors when they are reported
  (bind _returnvalue (UserInterface|CreateWidget "/Game/SplitTheParty/UI/WBP_InitialRumorReport.WBP_InitialRumorReport_C" self (Utilities|Array|MakeArray Agent) (CallFunction|DoAnyHeroesShowOverridesatAgentLocation Agent)))
  (CallFunction|ShowDialogBox _returnvalue))

(event Input|ActionEvents|InputActionQuit
  (params (Key :type Key%20Structure))
  (:Pressed
    (bind _returnvalue (UserInterface|CreateWidget "/Game/SplitTheParty/UI/WBP_QuitConfirm.WBP_QuitConfirm_C" self))
    (CallFunction|ShowDialogBox _returnvalue)))

(fn ConstructionScript)

(fn ShowDialogBox
  (params (Dialog :type WBP%20Dismissable%20Dialog%20Object%20Reference))
  (CallFunction|ZoomDialog Dialog)
  (LocalVariables|SetTheDialog Dialog)
  (Input|SetInputModeUIOnly self (LocalVariables|GetTheDialog) "DoNotLock")
  (EventDispatchers|BindEventtoOnDialogDismissed (LocalVariables|GetTheDialog) (EventDispatchers|CreateEvent :!event Custom|OnDialogDismissed))
  (UserInterface|Viewport|AddtoViewport (LocalVariables|GetTheDialog) 0))

(fn DoAnyHeroesShowOverridesatAgentLocation
  (params (Agent :type Agent%20Object%20Reference))
  (bind _returnvalue (Game|GetGameMode))
  (bind _asbp_game_mode (Utilities|Casting|CastToBP_GameMode _returnvalue))
  (for _array_element (Class|SplitthePartyGameMode|GetHeroesat _asbp_game_mode (Class|WorldMap|GetTile (Variables|/Script/SplitTheParty.SplitThePartyGameMode|GetWorldMap _asbp_game_mode) (Variables|/Script/SplitTheParty.Agent|GetHex Agent)))
    (if (Class|Hero|RevealsRumorOverrides _array_element)
      (return true)))
  (return false))