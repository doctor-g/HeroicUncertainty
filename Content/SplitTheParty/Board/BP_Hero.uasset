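; BP_Hero is the board piece for a hero in SplitTheParty, tinted with its own color.
; It binds to the game mode's turn-start event and makes its material glow only while it is the active hero.
; Moves play footsteps and animate the piece with a timeline lerp and height offset to an index-named socket on the target hex tile, then signal completion.
; Resting plays a fire sound.
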(event Custom|OnHeroStartTurn
  (params (Hero :type Hero%20Object%20Reference))
  ;[1 1 1] Watch the game mode for hero turn changes and glow when it's my turn.
  (Rendering|Material|SetScalarParameterValue (Variables|Default|GetMaterial) "Glow" (select (== Hero self) 1.0 0.0) :!class /Script/Engine.MaterialInstanceDynamic))

(event EventBeginPlay
  ;[1 1 1] Set up the player's color and material.
  (bind _returnvalue (Rendering|Material|CreateDynamicMaterialInstance (Variables|Default|GetCylinder) 0 "/Game/SplitTheParty/Board/M_Hero.M_Hero" "None" :!class /Script/Engine.PrimitiveComponent))
  (bind _output_get (Variables|Default|SetMaterial _returnvalue))
  (Rendering|Material|SetVectorParameterValue _output_get "Color" (Variables|Default|GetColor) :!class /Script/Engine.MaterialInstanceDynamic)
  ;[1 1 1] Watch the game mode for hero turn changes and glow when it's my turn.
  (bind _asbp_game_mode (Utilities|Casting|CastToBP_GameMode (Game|GetGameMode)))
  (EventDispatchers|BindEventtoOnHeroTurnStart _asbp_game_mode (delegate Custom|OnHeroStartTurn)))

(event EventRest
  (Audio|PlaySound2D "/Game/SplitTheParty/Audio/A_Fire.A_Fire" 1.0 1.0 0.0 0 0)
  (|CallParentFunction))

(event EventMoveto
  (params (Destination :type Hex%20Tile%20Object%20Reference))
  ;[1 1 1] MoveTo
  (Audio|PlaySound2D "/Game/SplitTheParty/Audio/A_Footsteps.A_Footsteps" 1.0 1.0 0.0 0 0)
  (Variables|Default|SetMovementStart (Transformation|GetActorLocation))
  (Variables|Default|SetMovementEnd (Transformation|GetSocketLocation (Variables|/Game/SplitTheParty/Board/BP_HexTile.BP_HexTile_C|GetHexMesh (.AsBP%20Hex%20Tile (Utilities|Casting|CastToBP_HexTile Destination))) (CallFunction|HexSocketName)))
  (|CallParentFunction Destination)
  (bind (_direction _alpha _zoffset) (Timeline|MovementAnimation PlayFromStart)
    (:Update
      (Transformation|SetActorLocation (Math|Vector|Lerp(Vector) (Math|Vector|MakeVector (.x (Variables|Default|GetMovementStart)) (.y (Variables|Default|GetMovementStart)) (+ _zoffset (.z (Variables|Default|GetMovementStart)))) (Math|Vector|MakeVector (.x (Variables|Default|GetMovementEnd)) (.y (Variables|Default|GetMovementEnd)) (+ _zoffset (.z (Variables|Default|GetMovementEnd)))) _alpha) false true))
    (:Finished
      (Default|CallOnHeroMovementComplete))))

(fn ConstructionScript)

(fn HexSocketName
  (return (Utilities|String|StringToName (Utilities|String|Append "Hero" (Utilities|String|ToString(Integer) (Variables|Default|GetIndex))))))