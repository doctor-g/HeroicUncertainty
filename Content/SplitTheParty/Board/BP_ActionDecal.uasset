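; BP_ActionDecal is a clickable board decal that represents an action and broadcasts it through an action-selected delegate when clicked.
; A dynamic material instance, created from a supplied material, drives the decal's tint and opacity.
; A Cube component handles cursor events, forwarding hover delegates and playing or reversing a glow timeline that blends the tint toward white.
; Show fades the decal in with an opacity timeline, and SetTint updates the base color.
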(event OnClicked(Cube)
  (params (TouchedComponent :type Primitive%20Component%20Object%20Reference) (ButtonPressed :type Key%20Structure))
  ;[1 1 1] On clicked: Call action selected delegate
  (Default|CallOnActionSelected (Variables|Default|GetAction)))

(event OnBeginCursorOver(Cube)
  (params (TouchedComponent :type Primitive%20Component%20Object%20Reference))
  ;[1 1 1] Glow the decal upon mouseover
  (Default|CallOnCustomBeginCursorOver self)
  (bind _alpha (Timeline|Glow PlayFromStart)
    (:Update
      (Rendering|Material|SetVectorParameterValue (Variables|Default|GetDecalMaterial) "Tint" (Math|Color|Lerp(LinearColor) (Variables|Default|GetTint) "(R=1.000000,G=1.000000,B=1.000000,A=1.000000)" _alpha) :!class /Script/Engine.MaterialInstanceDynamic))))

(event OnEndCursorOver(Cube)
  (params (TouchedComponent :type Primitive%20Component%20Object%20Reference))
  ;[1 1 1] Glow the decal upon mouseover
  (Default|CallOnCustomEndCursorOver self)
  (bind _alpha (Timeline|Glow ReverseFromEnd)
    (:Update
      (Rendering|Material|SetVectorParameterValue (Variables|Default|GetDecalMaterial) "Tint" (Math|Color|Lerp(LinearColor) (Variables|Default|GetTint) "(R=1.000000,G=1.000000,B=1.000000,A=1.000000)" _alpha) :!class /Script/Engine.MaterialInstanceDynamic))))

(event Custom|SetDecalBaseMaterial
  (params (Material :type Material%20Interface%20Object%20Reference))
  ;[1 1 1] SetDecalBaseMaterial
  (bind _returnvalue (Rendering|Material|CreateDynamicMaterialInstance Material "None" :!class /Script/Engine.KismetMaterialLibrary))
  (bind _output_get (Variables|Default|SetDecalMaterial _returnvalue))
  (Rendering|Components|Decal|SetDecalMaterial (Variables|Default|GetDecal) _output_get)
  (Rendering|Material|SetVectorParameterValue _output_get "Tint" (Variables|Default|GetTint) :!class /Script/Engine.MaterialInstanceDynamic))

(event Custom|Show
  ;[1 1 1] Show: Fade in the decal
  (bind _opacity (Timeline|ShowAnimation PlayFromStart)
    (:Update
      (Rendering|Material|SetScalarParameterValue (Variables|Default|GetDecalMaterial) "Opacity" _opacity :!class /Script/Engine.MaterialInstanceDynamic))))

(fn ConstructionScript)

(fn SetTint
  (params (Tint :type Linear%20Color%20Structure))
  (bind _output_get (Variables|Default|SetTint Tint))
  (Rendering|Material|SetVectorParameterValue (Variables|Default|GetDecalMaterial) "Tint" _output_get :!class /Script/Engine.MaterialInstanceDynamic))