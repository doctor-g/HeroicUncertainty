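; Clickable cone marker for a peril on the board that reopens the rumor report tied to it.
; A dynamic material created on BeginPlay drives a hover highlight through its Highlight parameter.
; Clicking creates a reminder rumor report widget from the reporting agents and shows it as a dialog through the player controller.
; The removal animation fades Opacity with a timeline, then signals that the animation is complete.
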(event OnClicked(Cone)
  (params (TouchedComponent :type Primitive%20Component%20Object%20Reference) (ButtonPressed :type Key%20Structure))
  (bind _returnvalue (UserInterface|CreateWidget "/Game/SplitTheParty/UI/WBP_ReminderRumorReport.WBP_ReminderRumorReport_C" (Game|GetPlayerController 0) (Class|PerilMarker|GetReportingAgents)))
  (Default|ShowDialogBox (.AsBP%20Player%20Controller (Utilities|Casting|CastToBP_PlayerController (Game|GetPlayerController 0))) _returnvalue))

(event OnBeginCursorOver(Cone)
  (params (TouchedComponent :type Primitive%20Component%20Object%20Reference))
  (Rendering|Material|SetScalarParameterValue (Variables|Default|GetMaterial) "Highlight" 1.0 :!class /Script/Engine.MaterialInstanceDynamic))

(event OnEndCursorOver(Cone)
  (params (TouchedComponent :type Primitive%20Component%20Object%20Reference))
  (Rendering|Material|SetScalarParameterValue (Variables|Default|GetMaterial) "Highlight" 0.0 :!class /Script/Engine.MaterialInstanceDynamic))

(event EventBeginPlay
  (bind _returnvalue (Rendering|Material|CreateDynamicMaterialInstance (Variables|Default|GetCone) 0 "/Game/SplitTheParty/Board/M_PerilMarker.M_PerilMarker" "None" :!class /Script/Engine.PrimitiveComponent))
  (Variables|Default|SetMaterial _returnvalue))

(event EventPlayRemovalAnimation
  (bind _opacity (Timeline|FadeOut PlayFromStart)
    (:Update
      (Rendering|Material|SetScalarParameterValue (Variables|Default|GetMaterial) "Opacity" _opacity :!class /Script/Engine.MaterialInstanceDynamic))
    (:Finished
      (Class|PerilMarker|NotifyAnimationComplete))))

(fn ConstructionScript)