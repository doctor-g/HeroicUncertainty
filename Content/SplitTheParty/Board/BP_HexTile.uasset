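; Board hex tile Blueprint that displays its name, optional coordinates and the hero actions available on it.
; Child-actor decals for Move, Quest and Rest are configured at construction, then shown for available actions in the current hero's color, forwarding selections to BP_GameMode through a ForEachActionDecal macro loop's bindings.
; Defilement plays a timeline that drives a dynamic material parameter, and a mesh socket supplies the peril marker transform.
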(event Custom|OnActionSelected
  (params (Action :type EHexAction%20Enum :default "Move"))
  ;[1 1 1] Set Tile Actions
  (Default|OnActionSelected (.AsBP%20Game%20Mode (Utilities|Casting|CastToBP_GameMode (Game|GetGameMode))) self Action))

(event Custom|OnTileDefilement
  (params (Tile :type Hex%20Tile%20Object%20Reference))
  ;[1 1 1] When this tile is defiled, update its material.
  (bind _percent (Timeline|DefileTimeline Play)
    (:Update
      (Rendering|Material|SetScalarParameterValue (Variables|Default|GetMaterial) "Defiled" _percent :!class /Script/Engine.MaterialInstanceDynamic))))

(event EventBeginPlay
  ;[1 1 1] BeginPlay: Configure the decal mouse hover events
  (for _array_element (Actor|GetComponentsByClass "/Script/Engine.ChildActorComponent")
    ;[1 1 1] Set up the mapping of actions to action decals
    (Utilities|Map|Add (Variables|Default|GetActionMap) "" (Variables|Default|GetMoveChild))
    (Utilities|Map|Add (Variables|Default|GetActionMap) "Quest" (Variables|Default|GetQuestChild))
    (Utilities|Map|Add (Variables|Default|GetActionMap) "Rest" (Variables|Default|GetRestChild))
    ;[1 1 1] Set up the dynamic material instance
    (bind _returnvalue (Rendering|Material|CreateDynamicMaterialInstance (Variables|Default|GetHexMesh) 0 "/Game/SplitTheParty/Board/M_Hex.M_Hex" "None" :!class /Script/Engine.PrimitiveComponent))
    (Variables|Default|SetMaterial _returnvalue)
    ;[1 1 1] When this tile is defiled, update its material.
    (EventDispatchers|BindEventtoOnTileDefiled (delegate Custom|OnTileDefilement))))

(event EventSetTileActions
  (params (Actions_ :type Array%20of%20EHexAction%20Enums :default "Move"))
  ;[1 1 1] Set Tile Actions
  (Variables|Default|SetPreviousActions (Variables|Default|GetActions))
  (|CallParentFunction Actions_)
  (bind (_component _actiondecal) (Utilities|ForEachActionDecal)
    (:LoopBody
      (Default|SetTint _actiondecal (CallFunction|GetCurrentHeroColor))
      (if (Utilities|Array|ContainsItem (Variables|Default|GetActions) (Variables|/Game/SplitTheParty/Board/BP_ActionDecal.BP_ActionDecal_C|GetAction _actiondecal))
        (Rendering|SetVisibility _component true false)
        (Default|Show _actiondecal)
        (EventDispatchers|BindEventtoOnActionSelected _actiondecal (delegate Custom|OnActionSelected))
        (else
          (Rendering|SetVisibility _component false false)
          (EventDispatchers|UnbindEventfromOnActionSelected _actiondecal (delegate Custom|OnActionSelected)))))))

(event EventSetCoordinates
  (params (Coords :type Hex%20Structure))
  (bind (_q _r) (Utilities|Struct|BreakHex Coords))
  (|CallParentFunction Coords)
  (Rendering|Components|TextRender|SetText (Variables|Default|GetCoords) (Utilities|Text|FormatText "({Q},{R})" _q _r)))

(event EventSetTileName
  (params (Name_ :type Text%20%28by%20ref%29))
  ;[1 1 1] Update the tile name as rendered when the name changes
  (|CallParentFunction Name_)
  (Rendering|Components|TextRender|SetText (Variables|Default|GetTextRender) Name_))

(event EventSetActionTint
  (params (Tint_ :type Linear%20Color%20Structure))
  ;[1 1 1] SetActionTint
  (|CallParentFunction Tint_))

(fn ConstructionScript
  (CallFunction|ConfigureChildActionDecal (Variables|Default|GetRestChild) "/Game/SplitTheParty/Board/MI_Rest.MI_Rest" "Rest")
  (CallFunction|ConfigureChildActionDecal (Variables|Default|GetQuestChild) "/Game/SplitTheParty/Board/MI_Quest.MI_Quest" "Quest")
  (CallFunction|ConfigureChildActionDecal (Variables|Default|GetMoveChild) "/Game/SplitTheParty/Board/MI_Move.MI_Move" "Move")
  (Rendering|SetVisibility (Variables|Default|GetCoords) (Variables|Default|GetbShowCoordinates) false))

(fn GetCurrentHeroColor
  (return (Variables|/Script/SplitTheParty.Hero|GetColor (Variables|/Script/SplitTheParty.SplitThePartyGameMode|GetCurrentHero (.AsBP%20Game%20Mode (Utilities|Casting|CastToBP_GameMode (Game|GetGameMode)))))))

(fn ConfigureChildActionDecal
  (params (Component :type Child%20Actor%20Component%20Object%20Reference) (Material :type Material%20Interface%20Object%20Reference) (Action :type EHexAction%20Enum :default "Move"))
  (LocalVariables|SetTheAction Action)
  (bind _asbp_action_decal (Utilities|Casting|CastToBP_ActionDecal (Variables|/Script/Engine.ChildActorComponent|GetChildActor Component))
    (:then
      (bind _output_get (LocalVariables|SetDecal _asbp_action_decal))
      (Default|SetDecalBaseMaterial _output_get Material)
      (Variables|/Game/SplitTheParty/Board/BP_ActionDecal.BP_ActionDecal_C|SetAction (LocalVariables|GetDecal) (LocalVariables|GetTheAction)))
    (:CastFailed
      (Development|PrintString "Unexpected decal actor class"))))

(fn GetPerilMarkerSocketTransform
  (return (Transformation|GetSocketTransform (Variables|Default|GetHexMesh) "Peril" "RTS_World")))