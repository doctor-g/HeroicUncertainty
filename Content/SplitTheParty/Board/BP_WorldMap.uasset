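; BP_WorldMap builds the game's hexagonal world map out of BP_HexTile child actors in its Construction Script.
; It loops over axial Q/R coordinates, keeping those within Radius of the origin, and positions each tile by converting its hex coordinates to a spaced relative location.
; Each tile receives its coordinates, a name found by LookupHexName's linear search of NameTable, and a back-reference, and is stored in HexTileMap by coordinate.
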(fn ConstructionScript
  (bind _radius (Variables|Configuration|GetRadius))
  (bind _returnvalue (- 0 _radius))
  ;[1 1 1] Iterate through all the tiles within Radius of the center
  (for _index (range _returnvalue _radius) ; Q
    (for _index_2 (range _returnvalue _radius) ; R
      (bind _output_get (LocalVariables|SetCoords (Utilities|Struct|MakeHex _index _index_2)))
      (if (<= (Class|HexBlueprintLibrary|Distance _output_get) (Variables|Configuration|GetRadius))
        (Utilities|FlowControl|Sequence
          (:then_0
            ;[1 1 1] Create the child actor component and configure the child hex tile
            (bind _returnvalue_2 (AddComponent|AddChildActorComponent false))
            (ChildActorComponent|SetChildActorClass _returnvalue_2 "/Game/SplitTheParty/Board/BP_HexTile.BP_HexTile_C")
            (bind _output_get_2 (LocalVariables|SetTile (.AsBP%20Hex%20Tile (Utilities|Casting|CastToBP_HexTile (Variables|/Script/Engine.ChildActorComponent|GetChildActor _returnvalue_2)))))
            (Class|HexTile|SetCoordinates _output_get_2 (LocalVariables|GetCoords))
            (Class|HexTile|SetTileName (LocalVariables|GetTile) (CallFunction|LookupHexName (LocalVariables|GetCoords))))
          (:then_1
            ;[1 1 1] Set the relative location of the child actor
            (Transformation|SetActorRelativeTransform (LocalVariables|GetTile) (Math|Transform|MakeTransform (Math|Vector|MakeVector (.x (* (Class|HexBlueprintLibrary|HextoUnitVector (LocalVariables|GetCoords)) (Variables|Configuration|GetDistanceBetweenHexCenters))) (.y (* (Class|HexBlueprintLibrary|HextoUnitVector (LocalVariables|GetCoords)) (Variables|Configuration|GetDistanceBetweenHexCenters))) 0.0) "0, 0, 0" "1,1,1") false true))
          (:then_2
            ;[1 1 1] Store the tile in the map for later reference and set its world to self
            (Utilities|Map|Add (Variables|Default|GetHexTileMap) (LocalVariables|GetCoords) (LocalVariables|GetTile))
            (Class|HexTile|SetWorldMap (LocalVariables|GetTile) self)))))))

(fn LookupHexName
  (params (Coords :type Hex%20Structure))
  (bind _nametable (Variables|Configuration|GetNameTable))
  (bind _outrownames (DataTable|GetDataTableRowNames _nametable))
  (for _array_element _outrownames
    (bind _returnvalue (Utilities|GetDataTableRow _nametable _array_element)
      (:then
        (if (== (.Hex (Utilities|Struct|BreakHexTileNameRow _returnvalue)) Coords)
          (return (.Name (Utilities|Struct|BreakHexTileNameRow _returnvalue)))))))
  (Development|PrintString "Tile name not found!"))